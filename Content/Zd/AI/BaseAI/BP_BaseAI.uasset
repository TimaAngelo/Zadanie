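; Base AI pawn that patrols, reacts to perceived actors and sounds, attacks, and is destroyed once its health runs out.
; Perception and movement events write state, enemy and target points to the Blackboard.
; Patrol points are random reachable locations around spawn; sound points are randomized around the stimulus receiver location.
; Attack runs a forward line trace and calls ApplyDamage, but the hit actor is not passed as its target.
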(event `MoveToLast`
  ;[1 1 1] LastSeeLocation
  (`BlackboardComponent.SetValueAsEnum` (`AIBlueprintHelperLibrary.GetBlackboard` null) "State" 0)
  (`|AIMoveTo` self (`self.LastEnemyLocation`) null
    (:`OnSuccess`
      (if (!= (`self.StateAI`) 3)
        (`BlackboardComponent.SetValueAsEnum` (`AIBlueprintHelperLibrary.GetBlackboard` null) "State" 1)))))

(event `self.ReceiveBeginPlay`
  ;[1 1 1] StartLocation
  (set `self.StartLocation` (`self.K2_GetActorLocation`)))

(event `StatePatrol`
  ;[1 1 1] StatePatrol
  (`BlackboardComponent.SetValueAsEnum` (`AIBlueprintHelperLibrary.GetBlackboard` null) "State" 1))

(event `self.AIPerception.OnPerceptionUpdated`
  (params (UpdatedActors :type "Array of Actor Object Reference (by ref)"))
  (bind _returnvalue (`AIBlueprintHelperLibrary.GetBlackboard` null))
  ;[1 1 1] AISee
  (for _array_element UpdatedActors
    (if (!= _array_element self)
      (`/Engine/EditorBlueprintResources/StandardMacros.IsValid` _array_element
        (:`Is Valid`
          (set `self.LastEnemyLocation` (`self.K2_GetActorLocation` _array_element))
          (`BlackboardComponent.SetValueAsObject` _returnvalue "Enemy" _array_element)
          (`BlackboardComponent.SetValueAsEnum` _returnvalue "State" 3)
          (break))))))

(event `AIPatrolPoint`
  ;[1 1 1] CreatePatrolPoint
  (set `self.StateAI` "NewEnumerator1")
  (bind _output_get (set `self.PatrolPoint` (`NavigationSystemV1.K2_GetRandomReachablePointInRadius` (`self.StartLocation`) 2000.0 null null)))
  (`BlackboardComponent.SetValueAsVector` (`AIBlueprintHelperLibrary.GetBlackboard` null) "PatrolPoint" _output_get))

(event `EventAttack`
  ;[1 1 1] Attack
  (`self.TraceFunction`)
  (`GameplayStatics.ApplyDamage` null (`self.Base Damage`) null self))

(event `self.ReceiveAnyDamage`
  (params (Damage :type "Float (single-precision)") (DamageType :type "DamageType Object Reference") (InstigatedBy :type "Controller Object Reference") (DamageCauser :type "Actor Object Reference"))
  ;[1 1 1] Damage And Deapth
  (if (> (`self.Health`) 0.0)
    (set `self.Health` (- (`self.Health`) Damage))
    (else
      (`self.K2_DestroyActor`))))

(event `self.AIPerception.OnTargetPerceptionUpdated`
  (params (Actor :type "Actor Object Reference") (Stimulus :type "AIStimulus Structure"))
  (bind (_age _expirationage _strength _stimuluslocation _receiverlocation _tag _bsuccessfullysensed) (break `AIStimulus` Stimulus))
  ;[1 1 1] Sound detect
  (if _bsuccessfullysensed
    (set `self.StateAI` "NewEnumerator2")
    (`BlackboardComponent.SetValueAsEnum` (`AIBlueprintHelperLibrary.GetBlackboard` null) "State" 2)
    (`BlackboardComponent.SetValueAsVector` (`AIBlueprintHelperLibrary.GetBlackboard` null) "SoundDetectPoint" (`NavigationSystemV1.K2_GetRandomReachablePointInRadius` _receiverlocation 1000.0 null null))))

(fn `TraceFunction`
  (returns (HitActor :type "Actor Object Reference"))
  (bind _returnvalue (`self.K2_GetActorLocation`))
  (bind (_outhit _returnvalue_2) (`KismetSystemLibrary.LineTraceSingle` _returnvalue (+ _returnvalue (* (`KismetMathLibrary.GetForwardVector` (`self.K2_GetActorRotation`)) 1000.0)) "TraceTypeQuery1"))
  (if _returnvalue_2
    (return (`.HitActor` (`GameplayStatics.BreakHitResult` _outhit)))))

(fn `UserConstructionScript`)