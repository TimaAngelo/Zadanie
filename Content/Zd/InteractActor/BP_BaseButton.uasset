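; BP_BaseButton is an interactable button that sends every BP_BaseAI in the level into patrol when pressed.
; Its Box trigger sets itself as the third-person character's InteractObject and enables CanPressButton on overlap, clearing both on exit.
; The Interact event gathers all BP_BaseAI actors and calls StatePatrol on each one.
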(event `/Game/Zd/Interface/BP_InteractInterface.Interact`
  ;[1 1 1] ActivateAI
  (bind _outactors (`GameplayStatics.GetAllActorsOfClass` "/Game/Zd/AI/BaseAI/BP_BaseAI.BP_BaseAI_C"))
  (for _array_element _outactors
    (bind _asbp_base_ai (cast `/Game/Zd/AI/BaseAI/BP_BaseAI` _array_element))
    (`/Game/Zd/AI/BaseAI/BP_BaseAI.StatePatrol` _asbp_base_ai)))

(event `self.Box.OnComponentBeginOverlap`
  (params (OverlappedComponent :type "PrimitiveComponent Object Reference") (OtherActor :type "Actor Object Reference") (OtherComp :type "PrimitiveComponent Object Reference") (OtherBodyIndex :type Integer) (bFromSweep :type Boolean) (SweepResult :type "HitResult Structure (by ref)"))
  ;[1 1 1] TriggerChek
  (bind _asbp_third_person_character (cast `/Game/ThirdPerson/Blueprints/BP_ThirdPersonCharacter` OtherActor))
  (set `/Game/ThirdPerson/Blueprints/BP_ThirdPersonCharacter.CanPressButton` true _asbp_third_person_character)
  (set `/Game/ThirdPerson/Blueprints/BP_ThirdPersonCharacter.InteractObject` self _asbp_third_person_character))

(event `self.Box.OnComponentEndOverlap`
  (params (OverlappedComponent :type "PrimitiveComponent Object Reference") (OtherActor :type "Actor Object Reference") (OtherComp :type "PrimitiveComponent Object Reference") (OtherBodyIndex :type Integer))
  ;[1 1 1] TriggerChek
  (bind _asbp_third_person_character (cast `/Game/ThirdPerson/Blueprints/BP_ThirdPersonCharacter` OtherActor))
  (set `/Game/ThirdPerson/Blueprints/BP_ThirdPersonCharacter.CanPressButton` false _asbp_third_person_character)
  (set `/Game/ThirdPerson/Blueprints/BP_ThirdPersonCharacter.InteractObject` null _asbp_third_person_character))

(fn `UserConstructionScript`)